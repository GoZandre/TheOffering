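; BP_DeerMask is an interactable deer mask that the first-person player picks up.
; On interaction it binds to the character's drop-object event, has the character grab the mask mesh, and plays a bark looked up from a data table row.
; When the drop event fires, it adds Quest_3 to the character, advancing the quest line.
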(event Custom|ActiveNextQuest
  (Default|AddQuest (stale EventInteractAction _asbp_first_person_character) "Quest_3"))

(event EventInteractAction
  (bind _barktoplay (Variables|Default|GetBarkToPlay))
  (bind (_datatable _rowname) (Utilities|Struct|BreakDataTableRowHandle _barktoplay))
  (|CallParentFunction)
  (bind _asbp_first_person_character (Utilities|Casting|CastToBP_FirstPersonCharacter (Game|GetPlayerCharacter 0)))
  (EventDispatchers|BindEventtoOnDropObject _asbp_first_person_character (delegate Custom|ActiveNextQuest))
  (Default|GrabObject _asbp_first_person_character (Variables|Default|GetDeerMaskMesh))
  (bind _returnvalue (Utilities|GetDataTableRow _datatable _rowname)
    (:then
      (Default|PlayBark _asbp_first_person_character _returnvalue))))

(fn ConstructionScript
  (|CallParentFunction))