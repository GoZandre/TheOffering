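; Base interactible actor that lets the first-person character trigger a linked event through an interaction collision.
; The collision starts query-enabled only if StartActive is set, and ActiveInteractible can enable it later.
; CreateInteraction and CancelInteraction bind and unbind InteractAction to the character's interact event.
; InteractAction disables the collision for single-use interactibles, then calls EventToDo if it is valid.
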(event Custom|InteractAction
  (bind _eventtodo (Variables|Default|GetEventToDo))
  (Utilities|FlowControl|Sequence
    (:then_0
      (if (Variables|Default|GetSingleInteraction)
        (Collision|SetCollisionEnabled (Variables|Default|GetInteractCollision) "NoCollision")))
    (:then_1
      (Utilities|IsValid _eventtodo
        (:Is%20Valid
          (Default|CallEvent _eventtodo))))))

(event Custom|CreateInteraction
  (params (FirstPersonCharacter :type BP%20First%20Person%20Character%20Object%20Reference))
  (EventDispatchers|BindEventtoInteractEvent FirstPersonCharacter (delegate Custom|InteractAction)))

(event Custom|CancelInteraction
  (params (FirstPersonCharacter :type BP%20First%20Person%20Character%20Object%20Reference))
  (EventDispatchers|UnbindEventfromInteractEvent FirstPersonCharacter (delegate Custom|InteractAction)))

(event Custom|ActiveInteractible
  (Collision|SetCollisionEnabled (Variables|Default|GetInteractCollision) "QueryOnly"))

(event EventBeginPlay
  (bind _interactcollision (Variables|Default|GetInteractCollision))
  (if (Variables|Default|GetStartActive)
    (Collision|SetCollisionEnabled _interactcollision "QueryOnly")
    (else
      (Collision|SetCollisionEnabled _interactcollision "NoCollision"))))

(fn ConstructionScript)