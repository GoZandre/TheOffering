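; BP_SewerDoor is an interactible sewer door that starts a cinematic when the first-person player overlaps its trigger after the door has been activated.
; It creates the W_Cinematic widget and binds that widget's mid-cinematic event to a teleport handler.
; The handler moves the player and view to a teleport point, then places either GoodNPC or BadNPC at NPCPos depending on whether the player has read the letter.
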(event OnComponentBeginOverlap(QuestAppearCollider)
  (params (OverlappedComponent :type Primitive%20Component%20Object%20Reference) (OtherActor :type Actor%20Object%20Reference) (OtherComp :type Primitive%20Component%20Object%20Reference) (OtherBodyIndex :type Integer) (bFromSweep :type Boolean) (SweepResult :type Hit%20Result%20Structure%20%28by%20ref%29))
  (bind _asbp_first_person_character (Utilities|Casting|CastToBP_FirstPersonCharacter OtherActor))
  (Variables|Default|SetAs%20BP%20First%20Person%20Character _asbp_first_person_character)
  (if (Variables|Default|GetCanInteract)
    (bind _returnvalue (UserInterface|CreateWidget "/Game/UserInterface/W_Cinematic.W_Cinematic_C" 0 (Variables|Default|GetAs%20BP%20First%20Person%20Character)))
    (EventDispatchers|BindEventtoMidCinematicEvent _returnvalue (delegate Custom|TeleportPlayer))
    (UserInterface|Viewport|AddtoViewport _returnvalue 10)))

(event Custom|TeleportPlayer
  (bind _cinematicteleportpoint (Variables|Default|GetCinematicTeleportPoint))
  (bind _npcpos (Variables|Default|GetNPCPos))
  (bind _returnvalue (Transformation|GetActorTransform _npcpos))
  (Transformation|SetActorLocation (Variables|Default|GetAs%20BP%20First%20Person%20Character) (Transformation|GetWorldLocation _cinematicteleportpoint) false false)
  (Pawn|SetControlRotation (Game|GetPlayerController 0) (Transformation|GetWorldRotation _cinematicteleportpoint))
  ;[0 0.09992 1] Je te laisse faire je sais pas comment tu veux gérer
  (if (Variables|/Game/FirstPerson/Blueprints/BP_FirstPersonCharacter.BP_FirstPersonCharacter_C|GetHaveReadTheLetter (Variables|Default|GetAs%20BP%20First%20Person%20Character))
    (Transformation|SetActorLocationAndRotation (Variables|Default|GetGoodNPC) (.location _returnvalue) (.rotation _returnvalue))
    (else
      (Transformation|SetActorLocationAndRotation (Variables|Default|GetBadNPC) (.location _returnvalue) (.rotation _returnvalue)))))

(event EventActiveInteractible
  (Variables|Default|SetCanInteract true))

(fn ConstructionScript
  (|CallParentFunction))