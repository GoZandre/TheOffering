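; Edgard's door, an interactible that responds differently to each successive interaction and leads into Quest_2.
; An interaction counter steps through a knock sound, a player bark from a data table, then a timeline swing open that adds the quest.
; Interaction collision is briefly disabled during knock and bark, and stays off once opened.
; An overlap collider shows a quest marker while interaction is enabled, removing it on exit or opening.
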(event OnComponentBeginOverlap(QuestAppearCollider)
  (params (OverlappedComponent :type Primitive%20Component%20Object%20Reference) (OtherActor :type Actor%20Object%20Reference) (OtherComp :type Primitive%20Component%20Object%20Reference) (OtherBodyIndex :type Integer) (bFromSweep :type Boolean) (SweepResult :type Hit%20Result%20Structure%20%28by%20ref%29))
  (if (Class|PrimitiveComponent|IsCollisionEnabled (Variables|Default|GetInteractCollision))
    (bind _asbp_first_person_character (Utilities|Casting|CastToBP_FirstPersonCharacter OtherActor))
    (bind _createdmarker02 (Default|CreateQuestMarker02 (Variables|/Game/FirstPerson/Blueprints/BP_FirstPersonCharacter.BP_FirstPersonCharacter_C|GetMainUserWidget _asbp_first_person_character) (Transformation|GetWorldLocation (Variables|Default|GetQuestAppearCollider))))))

(event OnComponentEndOverlap(QuestAppearCollider)
  (params (OverlappedComponent :type Primitive%20Component%20Object%20Reference) (OtherActor :type Actor%20Object%20Reference) (OtherComp :type Primitive%20Component%20Object%20Reference) (OtherBodyIndex :type Integer))
  (Utilities|Casting|CastToBP_FirstPersonCharacter OtherActor)
  (Utilities|IsValid (stale OnComponentBeginOverlap(QuestAppearCollider) _createdmarker02)
    (:Is%20Valid
      (Default|RemoveMarker (stale OnComponentBeginOverlap(QuestAppearCollider) _createdmarker02)))))

(event Custom|RemoveMarker
  (Utilities|IsValid (stale OnComponentBeginOverlap(QuestAppearCollider) _createdmarker02)
    (:Is%20Valid
      (Default|RemoveMarker (stale OnComponentBeginOverlap(QuestAppearCollider) _createdmarker02)))))

(event EventInteractAction
  (bind _interactionindex (Variables|Default|GetInteractionIndex))
  (bind _bark_01 (Variables|Default|GetBark_01))
  (bind (_datatable _rowname) (Utilities|Struct|BreakDataTableRowHandle _bark_01))
  (Utilities|FlowControl|Sequence
    (:then_0
      (switch int _interactionindex
        (:0
          (Audio|PlaySound2D "/Game/SoundEffect/KnockEffect.KnockEffect" 1.0 1.0 0.0 0 0)
          (Collision|SetCollisionEnabled (Variables|Default|GetInteractCollision) "NoCollision")
          (Utilities|FlowControl|Delay 1.0)
          (Collision|SetCollisionEnabled (Variables|Default|GetInteractCollision) "QueryOnly"))
        (:1
          (bind _asbp_first_person_character (Utilities|Casting|CastToBP_FirstPersonCharacter (Game|GetPlayerCharacter 0)))
          (Variables|Default|SetAs%20BP%20First%20Person%20Character _asbp_first_person_character)
          (bind _returnvalue (Utilities|GetDataTableRow _datatable _rowname)
            (:then
              (Default|PlayBark _asbp_first_person_character _returnvalue)
              (Collision|SetCollisionEnabled (Variables|Default|GetInteractCollision) "NoCollision")
              (Utilities|FlowControl|Delay (Variables|/Script/Engine.SoundBase|GetDuration (.VoiceLine (Utilities|Struct|BreakS_DialogSentence _returnvalue))))
              (Collision|SetCollisionEnabled (Variables|Default|GetInteractCollision) "QueryOnly"))))
        (:2
          (Collision|SetCollisionEnabled (Variables|Default|GetInteractCollision) "NoCollision")
          (CallFunction|RemoveMarker)
          (bind _opendoor (Timeline|OpenDoor PlayFromStart)
            (:Update
              (Transformation|SetRelativeRotation (Variables|Default|GetTheoffering_Door) (Math|Rotator|Lerp(Rotator) "0, 0, 0" "0.000000,-90.000000,0.000000" _opendoor) false false))
            (:Finished
              (Default|AddQuest (Variables|Default|GetAs%20BP%20First%20Person%20Character) "Quest_2"))))))
    (:then_1
      (Math|Integer|IncrementInt _interactionindex))))

(fn ConstructionScript
  (|CallParentFunction))