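; Interactible book in a house that tilts when used and opens a door, like a hidden switch.
; BeginPlay stores the start rotation, a target pitched 45 degrees from it, and the first BP_Door found in the level.
; InteractAction plays a timeline that lerps between the rotations; past a threshold, a DoOnce opens the door and plays an unlock sound.
; That branch also has an unused player character lookup and a "Camera Check" debug print.
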(event EventBeginPlay
  (bind _output_get (Variables|Default|SetRotaIni (Transformation|GetActorRotation)))
  (Variables|Default|SetRotaEnd (Math|Rotator|MakeRotator (.roll _output_get) (+ (.pitch _output_get) 45.0) (.yaw _output_get)))
  (bind _returnvalue (Actor|GetActorOfClass "/Game/FirstPerson/Blueprints/Leezak_Test/BP_Door.BP_Door_C"))
  (Variables|Default|SetDoor_Ref _returnvalue))

(event EventInteractAction
  (bind _newtrack_0 (Timeline|Timeline PlayFromStart)
    (:Update
      (if (> _newtrack_0 0.6)
        (Utilities|FlowControl|Sequence
          (:then_0
            (Utilities|FlowControl|DoOnce false
              (:Completed
                (Default|OpenDoor (Variables|Default|GetDoor_Ref))
                (Audio|PlaySound2D "/Game/FirstPerson/Blueprints/Leezak_Test/Ambiance/SC_Unlock.SC_Unlock" 1.0 1.0 0.0 0 0)
                (Actor|GetActorOfClass "/Game/FirstPerson/Blueprints/BP_FirstPersonCharacter.BP_FirstPersonCharacter_C")
                (Development|PrintString "Camera Check"))))
          (:then_1
            (Transformation|SetActorRotation (Math|Rotator|Lerp(Rotator) (Variables|Default|GetRotaIni) (Variables|Default|GetRotaEnd) _newtrack_0) :!label _label)))
        (else
          (goto _label))))))

(fn ConstructionScript
  (|CallParentFunction))