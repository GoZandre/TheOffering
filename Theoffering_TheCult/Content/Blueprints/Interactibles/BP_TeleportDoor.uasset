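; Interactible teleport door that moves the first-person character to the TPLoc component's location and turns player 0's control rotation to match it.
; Entering QuestAppearCollider caches the character for that teleport and creates a quest marker at the collider through the character's main user widget.
; Leaving the collider or calling RemoveMarker removes the marker if it is still valid.
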(event OnComponentBeginOverlap(QuestAppearCollider)
  (params (OverlappedComponent :type Primitive%20Component%20Object%20Reference) (OtherActor :type Actor%20Object%20Reference) (OtherComp :type Primitive%20Component%20Object%20Reference) (OtherBodyIndex :type Integer) (bFromSweep :type Boolean) (SweepResult :type Hit%20Result%20Structure%20%28by%20ref%29))
  (bind _asbp_first_person_character (Utilities|Casting|CastToBP_FirstPersonCharacter OtherActor))
  (Variables|Default|SetAs%20BP%20First%20Person%20Character _asbp_first_person_character)
  (bind _createdmarker02 (Default|CreateQuestMarker02 (Variables|/Game/FirstPerson/Blueprints/BP_FirstPersonCharacter.BP_FirstPersonCharacter_C|GetMainUserWidget _asbp_first_person_character) (Transformation|GetWorldLocation (Variables|Default|GetQuestAppearCollider)))))

(event OnComponentEndOverlap(QuestAppearCollider)
  (params (OverlappedComponent :type Primitive%20Component%20Object%20Reference) (OtherActor :type Actor%20Object%20Reference) (OtherComp :type Primitive%20Component%20Object%20Reference) (OtherBodyIndex :type Integer))
  (Utilities|Casting|CastToBP_FirstPersonCharacter OtherActor)
  (Utilities|IsValid (stale OnComponentBeginOverlap(QuestAppearCollider) _createdmarker02)
    (:Is%20Valid
      (Default|RemoveMarker (stale OnComponentBeginOverlap(QuestAppearCollider) _createdmarker02)))))

(event Custom|RemoveMarker
  (Utilities|IsValid (stale OnComponentBeginOverlap(QuestAppearCollider) _createdmarker02)
    (:Is%20Valid
      (Default|RemoveMarker (stale OnComponentBeginOverlap(QuestAppearCollider) _createdmarker02)))))

(event EventInteractAction
  (bind _tp_loc (Variables|Default|GetTP_Loc))
  (Transformation|SetActorLocation (Variables|Default|GetAs%20BP%20First%20Person%20Character) (Transformation|GetWorldLocation _tp_loc) false false)
  (Pawn|SetControlRotation (Game|GetPlayerController 0) (Transformation|GetWorldRotation _tp_loc)))

(fn ConstructionScript
  (|CallParentFunction))