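; BP_ConversationChanger is an events-system actor that switches an NPC's dialogue when triggered.
; Its CallEvent enables talking on NPCToChange and overwrites that NPC's quest-giver setting and starting sentence with NewQuestGiving and NewConversation.
; It then calls UpdateTalking on the NPC; the Blueprint has no other active logic, so it relies on an external caller to fire it.
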(event EventBeginPlay
  (|CallParentFunction) ; This node is disabled and will not be called.\nDrag off pins to build functionality.
)

(event Collision|EventActorBeginOverlap
  (params (OtherActor :type Actor%20Object%20Reference))
  (|CallParentFunction OtherActor) ; This node is disabled and will not be called.\nDrag off pins to build functionality.
)

(event EventTick
  (params (DeltaSeconds :type Float%20%28single-precision%29))
  (|CallParentFunction DeltaSeconds) ; This node is disabled and will not be called.\nDrag off pins to build functionality.
)

(event EventCallEvent
  (bind _npctochange (Variables|Default|GetNPCToChange))
  (Variables|/Game/Blueprints/NPCs/BP_Dialog_Npc.BP_Dialog_Npc_C|SetCanTalk _npctochange true)
  (Variables|/Game/Blueprints/NPCs/BP_Dialog_Npc.BP_Dialog_Npc_C|SetQuestGiver _npctochange (Variables|Default|GetNewQuestGiving))
  (Variables|/Game/Blueprints/NPCs/BP_Dialog_Npc.BP_Dialog_Npc_C|SetStartSentence _npctochange (Variables|Default|GetNewConversation))
  (Default|UpdateTalking _npctochange))

(fn ConstructionScript
  (|CallParentFunction))