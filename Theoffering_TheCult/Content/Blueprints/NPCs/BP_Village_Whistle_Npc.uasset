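; BP_Village_Whistle_Npc is a village NPC that, on StartEvent, plays looping audio-visual walking behavior toward a fixed world location.
; StartEvent starts the walking animation and audio, then issues an AI MoveTo; success and failure share the same follow-up.
; Unless Interupt is set, it plays a non-looping idle animation, waits, rechecks the flag and calls Walk, which is defined outside this graph.
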(event Custom|StartEvent
  (Components|Animation|PlayAnimation (Variables|Character|GetMesh) (Variables|Default|GetAnimation%20Walking) true)
  (Audio|Components|Audio|Play (Variables|Default|GetAudio) 0.0)
  (AI|AIMoveTo self "580.000000,2140.000000,118.000000" 0 1e+02 false
    (:OnSuccess
      _)
    (:OnFail
      _))
  (if (not (Variables|Default|GetInterupt))
    (Components|Animation|PlayAnimation (Variables|Character|GetMesh) (Variables|Default|GetAnimationIdle) false)
    (Utilities|FlowControl|Delay 1e+01)
    (if (not (Variables|Default|GetInterupt))
      (CallFunction|Walk))))

(fn ConstructionScript
  (|CallParentFunction))