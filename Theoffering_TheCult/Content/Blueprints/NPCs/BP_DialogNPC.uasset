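; BP_DialogNPC is an NPC that the player can start a dialog with.
; On BeginPlay it registers itself with its child BP_NpcDialog_Interactible actor and loops an optional base animation.
; StartDialog looks up the start sentence in a data table and passes it, with the NPC, to the first-person character's dialog.
; PlayAnim plays a one-shot animation, waits its length, then resumes the base loop.
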(event Custom|StartDialog
  (bind _startsentence (Variables|Default|GetStartSentence))
  (bind (_datatable _rowname) (Utilities|Struct|BreakDataTableRowHandle _startsentence))
  (bind _asbp_first_person_character (Utilities|Casting|CastToBP_FirstPersonCharacter (Game|GetPlayerCharacter 0)))
  (Variables|Default|SetAs%20BP%20First%20Person%20Character _asbp_first_person_character)
  (bind _returnvalue (Utilities|GetDataTableRow _datatable _rowname)
    (:then
      (Default|StartDialog (Variables|Default|GetAs%20BP%20First%20Person%20Character) self _returnvalue))
    (:RowNotFound
      (Development|PrintString "CANT FIND DT TABLE" true true "(R=1.000000,G=0.000000,B=0.017682,A=1.000000)"))))

(event Custom|PlayAnim
  (params (AnimToPlay :type Anim%20Sequence%20Object%20Reference))
  (bind _baseanimation (Variables|Default|GetBaseAnimation))
  (Components|Animation|PlayAnimation (Variables|Character|GetMesh) AnimToPlay false)
  (Utilities|FlowControl|Delay (Variables|/Script/Engine.AnimSequenceBase|GetSequenceLength AnimToPlay))
  (Utilities|IsValid _baseanimation
    (:Is%20Valid
      (Components|Animation|PlayAnimation (Variables|Character|GetMesh) _baseanimation true))))

(event EventBeginPlay
  (bind _baseanimation (Variables|Default|GetBaseAnimation))
  (bind _asbp_npc_dialog_interactible (Utilities|Casting|CastToBP_NpcDialog_Interactible (Variables|/Script/Engine.ChildActorComponent|GetChildActor (Variables|Default|GetNPC_Interaction))))
  (Variables|/Game/Blueprints/Interactibles/BP_NpcDialog_Interactible.BP_NpcDialog_Interactible_C|SetNpcToInteract _asbp_npc_dialog_interactible self)
  (Utilities|IsValid _baseanimation
    (:Is%20Valid
      (Components|Animation|PlayAnimation (Variables|Character|GetMesh) _baseanimation true))))

(fn ConstructionScript)