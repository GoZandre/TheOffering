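; BP_Dialog_Npc is a talkable NPC that starts dialogue with the first-person character and can hand out a quest.
; A child interactible actor targets it; dialogue and barks come from data table rows, alongside voiceline and animation playback.
; Entering its collider while a quest is pending shows a marker and plays a bark.
; Closing dialogue grants the quest once and disables interaction for unique dialogues.
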(event OnComponentBeginOverlap(QuestAppearCollider)
  (params (OverlappedComponent :type Primitive%20Component%20Object%20Reference) (OtherActor :type Actor%20Object%20Reference) (OtherComp :type Primitive%20Component%20Object%20Reference) (OtherBodyIndex :type Integer) (bFromSweep :type Boolean) (SweepResult :type Hit%20Result%20Structure%20%28by%20ref%29))
  (bind _enteringbark (Variables|Default|GetEnteringBark))
  (bind (_datatable _rowname) (Utilities|Struct|BreakDataTableRowHandle _enteringbark))
  (if (and (not (Utilities|Array|IsEmpty (Variables|Default|GetQuestGiver))) (Variables|Default|GetCanTalk))
    (Utilities|FlowControl|DoOnce false
      (:Completed
        (bind _asbp_first_person_character (Utilities|Casting|CastToBP_FirstPersonCharacter OtherActor))
        (bind _createdmarker (Default|CreateQuestMarker01 (Variables|/Game/FirstPerson/Blueprints/BP_FirstPersonCharacter.BP_FirstPersonCharacter_C|GetMainUserWidget _asbp_first_person_character) (Transformation|GetWorldLocation (Variables|Default|GetQuestAppearCollider))))
        (bind _returnvalue (Utilities|GetDataTableRow _datatable _rowname)
          (:then
            (Default|PlayBark _asbp_first_person_character _returnvalue)))))))

(event OnComponentEndOverlap(QuestAppearCollider)
  (params (OverlappedComponent :type Primitive%20Component%20Object%20Reference) (OtherActor :type Actor%20Object%20Reference) (OtherComp :type Primitive%20Component%20Object%20Reference) (OtherBodyIndex :type Integer))
  (bind _enteringbark (Variables|Default|GetEnteringBark))
  (bind (_datatable _rowname) (Utilities|Struct|BreakDataTableRowHandle _enteringbark))
  (Utilities|FlowControl|Sequence
    (:then_0
      (Utilities|Casting|CastToBP_FirstPersonCharacter OtherActor)
      (Utilities|IsValid (stale OnComponentBeginOverlap(QuestAppearCollider) _createdmarker)
        (:Is%20Valid
          (Default|RemoveMarker (stale OnComponentBeginOverlap(QuestAppearCollider) _createdmarker)))))
    (:then_1
      (Utilities|FlowControl|DoOnce false) ; enters at Reset
    )))

(event Custom|StartDialog
  (bind _startsentence (Variables|Default|GetStartSentence))
  (bind (_datatable _rowname) (Utilities|Struct|BreakDataTableRowHandle _startsentence))
  (bind _asbp_first_person_character (Utilities|Casting|CastToBP_FirstPersonCharacter (Game|GetPlayerCharacter 0)))
  (Variables|Default|SetAs%20BP%20First%20Person%20Character _asbp_first_person_character)
  (CallFunction|RemoveMarker)
  (bind _returnvalue (Utilities|GetDataTableRow _datatable _rowname)
    (:then
      (Default|StartDialog (Variables|Default|GetAs%20BP%20First%20Person%20Character) self _returnvalue))
    (:RowNotFound
      (Development|PrintString "CANT FIND DT TABLE" true true "(R=1.000000,G=0.000000,B=0.017682,A=1.000000)"))))

(event Custom|OnEndDialog
  (params (CurrentDialog :type S%20Dialog%20Sentence%20Structure))
  (bind _isclosingdialog (Utilities|Struct|BreakS_DialogSentence CurrentDialog))
  (Utilities|FlowControl|Sequence
    (:then_0
      (if _isclosingdialog
        (if (not (Utilities|Array|IsEmpty (Variables|Default|GetQuestGiver)))
          (Default|NewQuest (Variables|Default|GetAs%20BP%20First%20Person%20Character) (Variables|Default|GetQuestGiver))
          (Variables|Default|SetQuestGiver ""))))
    (:then_1
      (if (and (Variables|Default|GetIsUniqueDialog) _isclosingdialog)
        (Variables|Default|SetCanTalk false)
        (CallFunction|UpdateTalking)))))

(event Custom|RemoveMarker
  (Utilities|IsValid (stale OnComponentBeginOverlap(QuestAppearCollider) _createdmarker)
    (:Is%20Valid
      (Default|RemoveMarker (stale OnComponentBeginOverlap(QuestAppearCollider) _createdmarker)))))

(event Custom|PlayAnim
  (params (AnimToPlay :type Anim%20Sequence%20Object%20Reference))
  (bind _baseanimation (Variables|Default|GetBaseAnimation))
  (Components|Animation|PlayAnimation (Variables|Character|GetMesh) AnimToPlay false)
  (Utilities|FlowControl|Delay (Variables|/Script/Engine.AnimSequenceBase|GetSequenceLength AnimToPlay))
  (Utilities|IsValid _baseanimation
    (:Is%20Valid
      (Components|Animation|PlayAnimation (Variables|Character|GetMesh) _baseanimation true))))

(event Custom|UpdateTalking
  (bind _baseanimation (Variables|Default|GetBaseAnimation))
  (if (Variables|Default|GetCanTalk)
    (Variables|/Game/Blueprints/Interactibles/BP_NpcDialog_Interactible.BP_NpcDialog_Interactible_C|SetNpcToInteract (stale EventBeginPlay _asbp_npc_dialog_interactible) self)
    (Utilities|IsValid _baseanimation
      (:Is%20Valid
        (Components|Animation|PlayAnimation (Variables|Character|GetMesh) _baseanimation true)))
    (else
      (Collision|SetCollisionEnabled (Variables|/Game/Blueprints/Interactibles/BP_Interactible.BP_Interactible_C|GetInteractCollision (stale EventBeginPlay _asbp_npc_dialog_interactible)) "NoCollision"))))

(event Custom|PlayVoiceline
  (params (DialogSentence :type Sound%20Wave%20Object%20Reference))
  (Utilities|FlowControl|Sequence
    (:then_0
      (Utilities|IsValid (Variables|Default|GetCurrentSound)
        (:Is%20Valid
          (Audio|Components|Audio|Stop (Variables|Default|GetCurrentSound)))))
    (:then_1
      (bind _returnvalue (Audio|CreateSound2D DialogSentence 1.0 1.0 0.0 0))
      (bind _output_get (Variables|Default|SetCurrentSound _returnvalue))
      (Audio|Components|Audio|Play _output_get 0.0))))

(event EventBeginPlay
  (bind _baseanimation (Variables|Default|GetBaseAnimation))
  (bind _asbp_npc_dialog_interactible (Utilities|Casting|CastToBP_NpcDialog_Interactible (Variables|/Script/Engine.ChildActorComponent|GetChildActor (Variables|Default|GetNPC_Interaction))))
  (if (Variables|Default|GetCanTalk)
    (Variables|/Game/Blueprints/Interactibles/BP_NpcDialog_Interactible.BP_NpcDialog_Interactible_C|SetNpcToInteract _asbp_npc_dialog_interactible self)
    (Utilities|IsValid _baseanimation
      (:Is%20Valid
        (Components|Animation|PlayAnimation (Variables|Character|GetMesh) _baseanimation true)))
    (else
      (Collision|SetCollisionEnabled (Variables|/Game/Blueprints/Interactibles/BP_Interactible.BP_Interactible_C|GetInteractCollision _asbp_npc_dialog_interactible) "NoCollision"))))

(fn ConstructionScript)