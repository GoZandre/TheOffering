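; Village speaker NPC Blueprint that plays a voice line on request.
; Its PlayVoiceLine event stops VoiceLine if valid, then assigns the VoiceLineAtTrigger sound and plays it from the start.
; Nothing in this file calls the event, and the construction script only calls the parent.
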(event Custom|PlayVoiceLine
  (bind _voiceline (Variables|Default|GetVoiceLine))
  (bind _voiceline_2 (Variables|Default|GetVoiceLine))
  (Utilities|FlowControl|Sequence
    (:then_0
      (Utilities|IsValid _voiceline_2
        (:Is%20Valid
          (Audio|Components|Audio|Stop _voiceline_2))))
    (:then_1
      (Audio|Components|Audio|SetSound _voiceline (Variables|Default|GetVoiceLineAtTrigger))
      (Audio|Components|Audio|Play _voiceline 0.0))))

(event EventBeginPlay
  (|CallParentFunction) ; This node is disabled and will not be called.\nDrag off pins to build functionality.
)

(event Collision|EventActorBeginOverlap
  (params (OtherActor :type Actor%20Object%20Reference)))

(event EventTick
  (params (DeltaSeconds :type Float%20%28single-precision%29)))

(fn ConstructionScript
  (|CallParentFunction))