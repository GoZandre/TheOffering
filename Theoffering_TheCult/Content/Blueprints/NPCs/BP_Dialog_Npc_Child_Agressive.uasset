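; Aggressive dialog NPC child that becomes vulnerable once its dialog ends and can then be taken down once.
; On damage it plays an animation, then ragdolls and ignores Pawn collision after that animation's length.
; The same hit also fires OnKillEvent and calls ContinueQuestEvent on the first-person character.
; While it can talk, overlapping its QuestAppearCollider creates a quest marker, removed on end overlap or RemoveMarker.
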(event OnComponentBeginOverlap(QuestAppearCollider)
  (params (OverlappedComponent :type Primitive%20Component%20Object%20Reference) (OtherActor :type Actor%20Object%20Reference) (OtherComp :type Primitive%20Component%20Object%20Reference) (OtherBodyIndex :type Integer) (bFromSweep :type Boolean) (SweepResult :type Hit%20Result%20Structure%20%28by%20ref%29))
  (if (Variables|Default|GetCanTalk)
    (bind _asbp_first_person_character (Utilities|Casting|CastToBP_FirstPersonCharacter OtherActor))
    (bind _createdmarker02 (Default|CreateQuestMarker02 (Variables|/Game/FirstPerson/Blueprints/BP_FirstPersonCharacter.BP_FirstPersonCharacter_C|GetMainUserWidget _asbp_first_person_character) (Transformation|GetWorldLocation (Variables|Default|GetQuestAppearCollider))))))

(event OnComponentEndOverlap(QuestAppearCollider)
  (params (OverlappedComponent :type Primitive%20Component%20Object%20Reference) (OtherActor :type Actor%20Object%20Reference) (OtherComp :type Primitive%20Component%20Object%20Reference) (OtherBodyIndex :type Integer))
  (Utilities|Casting|CastToBP_FirstPersonCharacter OtherActor)
  (Utilities|IsValid (stale OnComponentBeginOverlap(QuestAppearCollider) _createdmarker02)
    (:Is%20Valid
      (Default|RemoveMarker (stale OnComponentBeginOverlap(QuestAppearCollider) _createdmarker02)))))

(event Custom|TakeDamage
  (bind _onkillevent (Variables|Default|GetOnKillEvent))
  (bind _damageanimation (Variables|Default|GetDamageAnimation))
  (if (Variables|Default|GetCanTakeDamage)
    (Variables|Default|SetCanTakeDamage false)
    (Components|Animation|PlayAnimation (Variables|Character|GetMesh) _damageanimation false)
    (Utilities|FlowControl|Sequence
      (:then_0
        (Utilities|FlowControl|Delay (Variables|/Script/Engine.AnimSequenceBase|GetSequenceLength _damageanimation))
        (Physics|SetSimulatePhysics (Variables|Character|GetMesh) true)
        (Collision|SetCollisionResponsetoChannel (Variables|Default|GetCapsuleComponent) "ECC_Pawn" "ECR_Ignore"))
      (:then_1
        (Utilities|IsValid _onkillevent
          (:Is%20Valid
            (Default|CallEvent _onkillevent))))
      (:then_2
        ;[0.331 1 0] New UPDATE !
        ;;[1 1 1] Oui j'ai la flemme de faire sa propre <3
        (bind _returnvalue (Actor|GetActorOfClass "/Game/FirstPerson/Blueprints/BP_FirstPersonCharacter.BP_FirstPersonCharacter_C"))
        (Default|ContinueQuestEvent _returnvalue)))))

(event EventBeginPlay
  (|CallParentFunction) ; This node is disabled and will not be called.\nDrag off pins to build functionality.
)

(event Collision|EventActorBeginOverlap
  (params (OtherActor :type Actor%20Object%20Reference)))

(event EventTick
  (params (DeltaSeconds :type Float%20%28single-precision%29)))

(event EventOnEndDialog
  (params (CurrentDialog :type S%20Dialog%20Sentence%20Structure))
  (|CallParentFunction CurrentDialog)
  (Variables|Default|SetCanTakeDamage true))

(event EventRemoveMarker
  (Utilities|IsValid (stale OnComponentBeginOverlap(QuestAppearCollider) _createdmarker02)
    (:Is%20Valid
      (Default|RemoveMarker (stale OnComponentBeginOverlap(QuestAppearCollider) _createdmarker02)))))

(fn ConstructionScript
  (|CallParentFunction))